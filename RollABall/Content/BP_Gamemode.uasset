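; Game mode that keeps a point score, shows it in a UI widget and signals a win at ten points.
; BeginPlay creates the widget and adds it to the viewport; UpdatePoints and ResetGame write the score into it.
; Each point gained runs EndGame, which raises the widget's Opacity variable and plays a 2D sound on reaching the target.
; The node that would set Opacity back to zero is unconnected.
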(event `self.ReceiveBeginPlay`
  (bind _returnvalue (`|CreateWidget` "/Game/ui.ui_C"))
  (bind _output_get (set `self.CurretUI` _returnvalue))
  (`UserWidget.AddToViewport` _output_get 0))

(event `Reset Game`
  (set `self.CurretPoints` 0)
  (set `/Game/ui.point` 0 (`self.CurretUI`)))

(event `Update Points`
  (bind _output_get (set `self.CurretPoints` (+ (`self.CurretPoints`) 1)))
  (set `/Game/ui.point` _output_get (`self.CurretUI`))
  (`self.End Game`))

(event `End Game`
  (if (== (`self.CurretPoints`) 10)
    (set `/Game/ui.opacity` 1.0 (`self.CurretUI`))
    (`GameplayStatics.PlaySound2D` "/Game/391539__unlistenable__electro-win-sound.391539__unlistenable__electro-win-sound" 1.0 1.0 0.0 null null)))

(fn `UserConstructionScript`)
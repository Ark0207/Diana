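; BP_Pickup is a collectible actor that awards points when the player touches it.
; On overlap with BP_Player it destroys itself, then calls UpdatePoints on BP_Gamemode and plays a 2D win jingle.
; It spins every Tick by adding a local rotation built from its RotX, RotY and RotZ variables, without delta-time scaling.
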(event `self.ReceiveActorBeginOverlap`
  (params (OtherActor :type "Actor Object Reference"))
  (cast `/Game/BP_Player` OtherActor)
  (`self.K2_DestroyActor`)
  (bind _asbp_gamemode (cast `/Game/BP_Gamemode` (`GameplayStatics.GetGameMode`)))
  (`/Game/BP_Gamemode.Update Points` _asbp_gamemode)
  (`GameplayStatics.PlaySound2D` "/Game/274179__littlerobotsoundfactory__jingle_win_synth_01.274179__littlerobotsoundfactory__jingle_win_synth_01" 1.0 1.0 0.0 null null))

(event `self.ReceiveTick`
  (params (DeltaSeconds :type "Float (single-precision)"))
  ;[1 1 1] PickUp
  (`self.K2_AddActorLocalRotation` (`KismetMathLibrary.MakeRotator` (`self.Rot X`) (`self.Rot Y`) (`self.Rot Z`))))

(fn `UserConstructionScript`)